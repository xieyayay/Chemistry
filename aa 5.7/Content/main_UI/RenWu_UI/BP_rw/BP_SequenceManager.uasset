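; Manager actor that plays equipment Level Sequences one at a time in a chemistry game with an exam mode.
; PlayLevelSequence clears the score widget hint, starts playback, immediately calls the task manager's OnSequenceCompleted, and optionally updates guide actors by equipment ID.
; Requests during playback only show a please-wait HUD tip.
; The finish callback, gated by a re-armed DoOnce, releases the lock, plays audio outside exam mode and opens the supplied widget.
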(event `self.ReceiveBeginPlay`)

(event `PlayLevelSequence`
  (params (SequenceAsset :type "LevelSequence Object Reference") (EquipmentID :type Integer) (UI_Widget :type "UserWidget Class Reference") (image :type "Texture2D Object Reference") (sound :type "SoundBase Object Reference") (zhi_yin :type Boolean))
  ;[1 1 1] 清空考试模式下的文本提示
  (bind _foundwidgets (`WidgetBlueprintLibrary.GetAllWidgetsOfClass` "/Game/Game_MoShi/WBP_score.WBP_score_C"))
  (`/Game/Game_MoShi/WBP_score.Give Tishi` _foundwidgets "")
  (if (not (`self.bIsPlaying`))
    (bind _outactor (`LevelSequencePlayer.CreateLevelSequencePlayer` SequenceAsset (make `MovieSceneSequencePlaybackSettings` false (struct) 1.0 0.0 false false false false false false "ForceKeepState")))
    (bind _output_get (set `self.CurrentSequenceActor` _outactor))
    (bind _sequenceplayer (`LevelSequenceActor.SequencePlayer` _output_get))
    (add `MovieSceneSequencePlayer.OnFinished` _sequenceplayer (delegate `OnSequenceFinished`))
    (`MovieSceneSequencePlayer.Play` _sequenceplayer)
    (set `self.bIsPlaying` true)
    (`|ExecutionSequence`
      (:`then_0`
        (`/Game/main_UI/RenWu_UI/BP_rw/BP_TaskManager1.On Sequence Completed` (`self.TaskManagerRef`))
        (bind _output_get_2 (set `self.CurrentEquipmentID` EquipmentID))
        (if zhi_yin
          (bind _outactors (`GameplayStatics.GetAllActorsOfClass` "/Game/model/New_add/material/BP_zhiyin1.BP_zhiyin1_C"))
          (for _array_element _outactors
            (`/Game/model/New_add/material/BP_zhiyin1.更新指引` _array_element _output_get_2))))
      (:`then_1`
        (goto _label :!via `Reset`)))
    (else
      (`/Game/main_UI/RenWu_UI/WBP_TaskPanel2.clicked_tips` (`/Game/main_UI/RenWu_UI/BP_rw/BP_TaskManager1.HUDWidgetRef` (`self.TaskManagerRef`)) (`|FormatText` "已点击{仪器}，请稍等" _)))))

(event `OnSequenceFinished`
  (`/Engine/EditorBlueprintResources/StandardMacros.DoOnce` false :!label _label
    (:`Completed`
      (set `self.bIsPlaying` false)
      (if (not (`/Game/Game_MoShi/BP_ChemistryGameInstance.IsExamMode` (cast `/Game/Game_MoShi/BP_ChemistryGameInstance` (`GameplayStatics.GetGameInstance`) :!pure true)))
        (`GameplayStatics.PlaySoundAtLocation` (stale `PlayLevelSequence` sound) (`self.K2_GetActorLocation`) (struct) 1.0 1.0 0.0 null null null null) ; 播放音频
      )
      (`/Engine/EditorBlueprintResources/StandardMacros.IsValid` (`self.TaskManagerRef`)
        (:`Is Valid`
          (if (`KismetSystemLibrary.IsValidClass` (stale `PlayLevelSequence` UI_Widget))
            (bind _returnvalue (`|CreateWidget` (stale `PlayLevelSequence` UI_Widget) (`GameplayStatics.GetPlayerController` 0)))
            (`UserWidget.AddToViewport` _returnvalue 100)))))))

(fn `UserConstructionScript`)
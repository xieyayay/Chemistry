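; BP_KT is an air-conditioner actor that shows its control widget component when something overlaps its trigger Box.
; Begin overlap waits briefly, reveals the Widget and plays the Kongtiao sound at the world origin rather than at the actor.
; End overlap hides the Widget after a longer delay, leaving the sound untouched.
; Neither event filters which actor triggers it.
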(event `self.Box.OnComponentBeginOverlap`
  (params (OverlappedComponent :type "PrimitiveComponent Object Reference") (OtherActor :type "Actor Object Reference") (OtherComp :type "PrimitiveComponent Object Reference") (OtherBodyIndex :type Integer) (bFromSweep :type Boolean) (SweepResult :type "HitResult Structure (by ref)"))
  ;[1 1 1] 空调控件组件的相关变化事件
  (`/Engine/EditorBlueprintResources/StandardMacros.IsValid` (`self.Box`)
    (:`Is Valid`
      (bind _widget (`self.Widget`)
        (:`then`
          (`KismetSystemLibrary.Delay` 0.5)
          (`SceneComponent.SetVisibility` _widget true false)
          (`GameplayStatics.PlaySoundAtLocation` "/Game/Deepseek/Sound_TS/kongtiao.kongtiao" (0.0 0.0 0.0) (struct) 1.0 1.0 0.0 null null null null))
        (:`else`)))))

(event `self.Box.OnComponentEndOverlap`
  (params (OverlappedComponent :type "PrimitiveComponent Object Reference") (OtherActor :type "Actor Object Reference") (OtherComp :type "PrimitiveComponent Object Reference") (OtherBodyIndex :type Integer))
  ;[1 1 1] 空调控件组件的相关变化事件
  (`/Engine/EditorBlueprintResources/StandardMacros.IsValid` (`self.Box`)
    (:`Is Valid`
      (`self.Widget`
        (:`then`
          (`KismetSystemLibrary.Delay` 1.0)
          (`SceneComponent.SetVisibility` (stale `self.Box.OnComponentBeginOverlap` _widget) false false))
        (:`else`)))))

(fn `UserConstructionScript`)
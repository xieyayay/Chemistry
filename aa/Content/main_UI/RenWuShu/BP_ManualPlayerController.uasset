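; BP_ManualPlayerController is a player controller Blueprint meant to toggle the RW_Book manual widget with the ShowManual input action.
; Pressing the action creates an RW_Book widget only when IsManualShowing is true, and does not add it to the viewport.
; The logic that adds or removes the stored widget instance and updates the flag is disconnected and never runs.
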(event `InputAction|ShowManual`
  (params (Key :type "Key Structure"))
  (:`Pressed`
    (if (`self.bIsManualShowing`)
      (bind _returnvalue (`|CreateWidget` "/Game/main_UI/RenWuShu/RW_Book.RW_Book_C" self)))))

(fn `UserConstructionScript`)
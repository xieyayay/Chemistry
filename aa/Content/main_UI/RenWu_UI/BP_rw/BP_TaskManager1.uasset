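; Task manager actor for a step-by-step equipment operation exercise, driven by an array of task structs.
; Equipment clicks are checked against the current step's single equipment/part or ordered ID list; wrong single-step clicks deduct score and show a tip.
; Completed steps play a level sequence through the sequence manager, and a completion handler advances the step.
; It also updates HUD hints and images, supports stepping back, and makes floating hints follow the mouse.
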(event `self.ReceiveBeginPlay`
  (bind _returnvalue (`GameplayStatics.GetActorOfClass` "/Game/ThirdPerson/Blueprints/BP_ThirdPersonGameMode.BP_ThirdPersonGameMode_C"))
  (set `self.BP Third Person Mode` _returnvalue))

(event `self.ReceiveTick`
  (params (DeltaSeconds :type "Float (single-precision)"))
  (bind (_locationx _locationy) (`PlayerController.GetMousePosition` (`GameplayStatics.GetPlayerController` 0)))
  (bind _txt_floatinghint (`/Game/main_UI/RenWu_UI/WBP_TaskPanel2.Txt_FloatingHint` (`self.HUDWidgetRef`)))
  (if (`|EnumEquality` (`Widget.GetVisibility` _txt_floatinghint) "Visible")
    (`Widget.SetRenderTranslation` _txt_floatinghint (`KismetMathLibrary.MakeVector2D` (+ _locationx 260.0) (+ _locationy 130.0)))))

(fn `CompleteCurrentStep`
  (bind (_stepnumber _taskdescription _targetequipmentid _targetequipmentids _targetpartid _targetsequence _biscompleted _bismultistep _currentclickindex _operationname _ui_widget _image _sound _zhi_yin) (break `/Game/main_UI/RenWu_UI/BP_rw/S_TaskStep` (`|GetArrayItem` (`self.Tasks`) (- (`self.CurrentTaskStep`) 1))))
  (set `self.Is Completed` true)
  (`self.UpdateTaskHint`)
  (`/Engine/EditorBlueprintResources/StandardMacros.IsValid` _targetsequence
    (:`Is Valid`
      (`/Game/main_UI/RenWu_UI/BP_rw/BP_SequenceManager.PlayLevelSequence` (`self.SequenceManagerRef`) _targetsequence _targetequipmentid _ui_widget null _sound _zhi_yin))))

(fn `ExecuteCurrentStepOperation`
  (bind _sequencemanagerref (`self.SequenceManagerRef`))
  (bind (_stepnumber _taskdescription _targetequipmentid _targetequipmentids _targetpartid _targetsequence _biscompleted _bismultistep _currentclickindex _operationname _ui_widget _image _sound _zhi_yin) (break `/Game/main_UI/RenWu_UI/BP_rw/S_TaskStep` (`|GetArrayItem` (`self.Tasks`) (- (`self.CurrentTaskStep`) 1))))
  (if (and (not _biscompleted) (`KismetSystemLibrary.IsValid` _targetsequence))
    (`/Game/main_UI/RenWu_UI/WBP_TaskPanel2.Show Task Image` (`/Game/ThirdPerson/Blueprints/BP_ThirdPersonGameMode.HUDWidget` (`self.BP Third Person Mode`)) _image) ; 单步图片播放
    (if (`KismetSystemLibrary.IsValid` _sequencemanagerref)
      (`/Game/main_UI/RenWu_UI/BP_rw/BP_SequenceManager.PlayLevelSequence` _sequencemanagerref _targetsequence _targetequipmentid _ui_widget null _sound _zhi_yin)
      (else
        (`KismetSystemLibrary.PrintString` "SequenceManagerRef无效")))
    (else
      (`KismetSystemLibrary.PrintString` "条件判断为假，不播放"))))

(fn `Go to Previous Step`
  (if (> (`self.CurrentTaskStep`) 1)
    (`/Engine/EditorBlueprintResources/StandardMacros.DecrementInt` (`self.CurrentTaskStep`)
      (:`  `
        (set `self.Is Completed` false)
        (set `self.Current Click Index` 0)
        (`self.UpdateTaskHint`)
        (`/Game/main_UI/RenWu_UI/WBP_TaskPanel2.Show Task Image` (`/Game/ThirdPerson/Blueprints/BP_ThirdPersonGameMode.HUDWidget` (`self.BP Third Person Mode`)) (`.image_58_19E5BDDB40673D8DF7D746801C2292D2` (break `/Game/main_UI/RenWu_UI/BP_rw/S_TaskStep` (`|GetArrayItem` (`self.Tasks`) (- (`self.CurrentTaskStep`) 1))))) ; 多步图片播放
      ))))

(fn `HandleEquipmentInteract`
  (params (Equipment :type "/Game/UI/BP/interact/BP_l/BP_interact Object Reference") (PartID :type Integer))
  (locals (EquipmentID :type "/Game/UI/BP/interact/BP_l/BP_interact Object Reference") (NewLocalVar :type Boolean))
  (bind _equipmentid (`/Game/UI/BP/interact/BP_l/BP_interact.EquipmentID` Equipment))
  (bind _returnvalue (- (`self.CurrentTaskStep`) 1))
  (bind _output (`|GetArrayItem` (`self.Tasks`) _returnvalue))
  (bind (_stepnumber _taskdescription _targetequipmentid _targetequipmentids _targetpartid _targetsequence _biscompleted _bismultistep _currentclickindex _operationname _ui_widget _image _sound _zhi_yin _membervar_66) (break `/Game/main_UI/RenWu_UI/BP_rw/S_TaskStep` _output))
  (`KismetSystemLibrary.PrintString` (`KismetTextLibrary.Conv_TextToString` (`|FormatText` "当前步骤{0}, 已点击ID{1}, bIsCompleted={2}" _stepnumber _equipmentid _biscompleted)) true true (struct :`G` 0.66 :`B` 1.0 :`A` 1.0) 3.0)
  (`/Engine/EditorBlueprintResources/StandardMacros.IsValid` (`local.Equipment`)
    (:`Is Valid`
      (set `self.Current Click Index` _currentclickindex)
      (bind _output_get (set `self.Is Completed` _biscompleted))
      (if _output_get
        (return)
        (else
          (bind _output_get_2 (set `self.Is Multi Step` _bismultistep))
          (if _output_get_2
            (if (< _currentclickindex (`KismetArrayLibrary.Array_Length` _targetequipmentids))
              (if (== _equipmentid (`|GetArrayItem` _targetequipmentids _currentclickindex))
                ;[1 1 1] click index回调结构体中
                (bind _output_get_3 (set `self.Current Click Index` (+ (`self.Current Click Index`) 1)))
                (bind _structout (setmembers `/Game/main_UI/RenWu_UI/BP_rw/S_TaskStep` :`StructRef` _output :`CurrentClickIndex` _output_get_3))
                (`KismetArrayLibrary.Array_Set` (`|MakeArray` _output) _returnvalue _structout)
                (`/Game/main_UI/RenWu_UI/WBP_TaskPanel2.Show Task Image` (`/Game/ThirdPerson/Blueprints/BP_ThirdPersonGameMode.HUDWidget` (`self.BP Third Person Mode`)) (`BlueprintMapLibrary.Map_Find` _membervar_66 _currentclickindex)) ; 多步图片播放
                ;[1 1 1] 点击指定一起后最终播放（依次点击后播放一次
                (if (>= _currentclickindex (`KismetArrayLibrary.Array_Length` _targetequipmentids))
                  (`self.CompleteCurrentStep` :!pinned true) ; 多步完结
                  (else
                    (`self.UpdateTaskHint`))))
              (else
                (return)))
            (elif (and (`KismetStringLibrary.EqualEqual_StrStr` (`KismetStringLibrary.Conv_IntToString` _equipmentid) (`KismetStringLibrary.Conv_IntToString` _targetequipmentid)) (or (== _targetpartid 0) (== PartID _targetpartid)))
              (`KismetSystemLibrary.PrintString` (`KismetTextLibrary.Conv_TextToString` (`|FormatText` "点击ID={0}, 要求ID={1}" _equipmentid _targetequipmentid)))
              (`self.CompleteCurrentStep` :!pinned true) ; 单步判断完成
              (`KismetSystemLibrary.PrintString` (`KismetStringLibrary.Conv_IntToString` (`self.CurrentTaskStep`)))
              (else
                ;[1 1 1] 考试模式
                (`KismetSystemLibrary.PrintString` "ID不满足")
                (bind _foundwidgets (`WidgetBlueprintLibrary.GetAllWidgetsOfClass` "/Game/Game_MoShi/WBP_score.WBP_score_C"))
                (bind `_当前总分` (`/Game/Game_MoShi/WBP_score.UpdateScoreDisplay` _foundwidgets 1))
                (`/Game/Game_MoShi/WBP_score.current_koufen` _foundwidgets 1)
                (`/Game/Game_MoShi/WBP_score.Give Tishi` _foundwidgets (`KismetTextLibrary.Conv_TextToString` _taskdescription))
                (if (<= `_当前总分` 0)
                  (`/Game/Game_MoShi/WBP_score.创建0分失败控件` _foundwidgets))))))))))

(fn `HideOperationHint`
  (`/Game/main_UI/RenWu_UI/WBP_TaskPanel2.HideFloatingHint` (`self.HUDWidgetRef`)))

(fn `On Sequence Completed`
  (set `self.CurrentTaskStep` (+ (`self.CurrentTaskStep`) 1))
  (`KismetSystemLibrary.PrintString` (`KismetTextLibrary.Conv_TextToString` (`|FormatText` "下一个步骤：{1}" (`self.CurrentTaskStep`))))
  (if (<= (`self.CurrentTaskStep`) (`KismetArrayLibrary.Array_Length` (`self.Tasks`)))
    (`self.UpdateTaskHint`)
    (else
      (`KismetSystemLibrary.PrintString` "所有任务完成，显示结束语"))))

(fn `ShowOperationHint`
  (params (Equipment :type "/Game/UI/BP/interact/BP_l/BP_interact Object Reference"))
  (bind (_stepnumber _taskdescription _targetequipmentid _targetequipmentids _targetpartid _targetsequence _biscompleted _bismultistep _currentclickindex _operationname) (break `/Game/main_UI/RenWu_UI/BP_rw/S_TaskStep` (`|GetArrayItem` (`self.Tasks`) (- (`self.CurrentTaskStep`) 1))))
  (if (and (`KismetStringLibrary.EqualEqual_StrStr` (`KismetStringLibrary.Conv_IntToString` (`/Game/UI/BP/interact/BP_l/BP_interact.EquipmentID` Equipment)) (`KismetStringLibrary.Conv_IntToString` _targetequipmentid)) (not _biscompleted))
    (`/Game/main_UI/RenWu_UI/WBP_TaskPanel2.ShowFloatingHint` (`self.HUDWidgetRef`) _operationname)))

(fn `UpdateTaskHint`
  (bind _hudwidgetref (`self.HUDWidgetRef`))
  (bind (_stepnumber _taskdescription _targetequipmentid _targetequipmentids _targetpartid _targetsequence _biscompleted _bismultistep _currentclickindex) (break `/Game/main_UI/RenWu_UI/BP_rw/S_TaskStep` (`|GetArrayItem` (`self.Tasks`) (- (`self.CurrentTaskStep`) 1))))
  (`/Engine/EditorBlueprintResources/StandardMacros.IsValid` (`self.HUDWidgetRef`)
    (:`Is Valid`
      (if _biscompleted
        (`/Game/main_UI/RenWu_UI/WBP_TaskPanel2.Set Task Hint Text` _hudwidgetref _taskdescription :!label _label)
        (elif _bismultistep
          (for _array_element (`self.EquipmentRefs`)
            (if (== (`/Game/UI/BP/interact/BP_l/BP_interact.EquipmentID` _array_element) (`|GetArrayItem` _targetequipmentids _currentclickindex))
              (bind _name (`/Game/UI/BP/interact/BP_l/BP_interact.GetEquipmentName` _array_element))
              (`/Game/main_UI/RenWu_UI/WBP_TaskPanel2.Set Task Hint Text` _hudwidgetref (`|FormatText` "步骤{0}，请点击{仪器名称}" _stepnumber _name))))
          (else
            (goto _label)))))
    (:`Is Not Valid`
      (return))))

(fn `UserConstructionScript`)
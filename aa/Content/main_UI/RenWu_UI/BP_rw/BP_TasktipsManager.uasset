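; Task-tips manager actor that tracks the current task and step from DT_Taskstips and broadcasts changes through event dispatchers.
; UpdateUI picks the current step's text from fixed row columns and fires OnTaskUpdated, except for Step18, which only sets the text.
; AdvanceStep increments steps, then calls NextTask to move along row names and fire OnTaskCompleted under a hard-coded index limit.
; GoToPreviousStepTips decrements the step, refreshing only when it still exceeds TotalSteps.
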(event `self.ReceiveBeginPlay`)

(fn `AdvanceStep`
  (bind _currentstep (`self.CurrentStep`))
  (bind _returnvalue (`|GetDataTableRow` "/Game/main_UI/RenWu_UI/BP_rw/DT_Taskstips.DT_Taskstips" (`self.CurrentTaskRow`))
    (:`then`
      (bind (_text _color _tasktitle _step1 _step2 _step3 _step4 _step5 _step6 _step7 _step8 _step9 _step10 _step11 _step12 _step13 _step14 _step15 _step16 _step17 _step18 _totalsteps) (break `/Game/main_UI/RenWu_UI/BP_rw/Message_Struct` _returnvalue))
      (if (< _currentstep _totalsteps)
        (set `self.CurrentStep` (+ 1 (`self.CurrentStep`)))
        (`self.Update UI`)
        (return)
        (elif (== _currentstep _totalsteps)
          (`self.NextTask`)
          (`self.Update UI`)
          (return))))))

(fn `Go to Previous Step(tips`
  (if (> (`self.CurrentStep`) 1)
    (bind _output_get (set `self.CurrentStep` (- (`self.CurrentStep`) 1)))
    (bind _returnvalue (`|GetDataTableRow` "/Game/main_UI/RenWu_UI/BP_rw/DT_Taskstips.DT_Taskstips" (`self.CurrentTaskRow`))
      (:`then`
        (if (> _output_get (`.TotalSteps_34_F441ED6F4215FA1EDB6E959408FF52B5` (break `/Game/main_UI/RenWu_UI/BP_rw/Message_Struct` _returnvalue)))
          (set `self.CurrentTaskIndex` (- (`self.NextIndex`) 1))
          (set `self.CurrentStep` 1)
          (`self.Update UI`))))))

(fn `NextTask`
  (bind _returnvalue (`|GetDataTableRow` "/Game/main_UI/RenWu_UI/BP_rw/DT_Taskstips.DT_Taskstips" (`self.CurrentTaskRow`))
    (:`then`
      (bind _outrownames (`DataTableFunctionLibrary.GetDataTableRowNames` "/Game/main_UI/RenWu_UI/BP_rw/DT_Taskstips.DT_Taskstips"))
      (if (< (`KismetArrayLibrary.Array_Find` _outrownames (`self.CurrentTaskRow`)) (`KismetArrayLibrary.Array_Length` _outrownames))
        (set `self.CurrentTaskRow` (`|GetArrayItem` _outrownames (`self.NextIndex`)))
        (set `self.CurrentStep` 1)
        (`self.Update UI`)
        (for (_array_element _array_index) _outrownames
          (if (== _array_element (`self.CurrentTaskRow`))
            (set `self.CurrentTaskIndex` _array_index)
            (break)))
        (bind _result (`/Engine/EditorBlueprintResources/StandardMacros.IncrementFloat` (`KismetMathLibrary.Conv_IntToDouble` (`self.CurrentTaskIndex`)))
          (:`  `
            (bind _output_get (set `self.NextIndex` (`KismetMathLibrary.FTrunc` _result)))
            (if (< _output_get 14)
              (`self.OnTaskCompleted` (`.text_35_E2251B3F4D841A138FEBA8B6BD7BC96A` (break `/Game/main_UI/RenWu_UI/BP_rw/Message_Struct` _returnvalue)))
              (`KismetSystemLibrary.PrintString` "完成一步！！！！！！"))))
        (else
          (`KismetSystemLibrary.PrintString` "所有任务已完成"))))))

(fn `Update UI`
  (bind _returnvalue (`|GetDataTableRow` "/Game/main_UI/RenWu_UI/BP_rw/DT_Taskstips.DT_Taskstips" (`self.CurrentTaskRow`))
    (:`then`
      (switch `int` (`self.CurrentStep`)
        (:`1`
          (bind (_text _color _tasktitle _step1 _step2 _step3 _step4 _step5 _step6 _step7 _step8 _step9 _step10 _step11 _step12 _step13 _step14 _step15 _step16 _step17 _step18) (break `/Game/main_UI/RenWu_UI/BP_rw/Message_Struct` _returnvalue))
          (set `self.CurrentStepText` _step1)
          (`self.OnTaskUpdated` _tasktitle (`self.CurrentStepText`) :!label _label))
        (:`2`
          (set `self.CurrentStepText` _step2)
          (goto _label))
        (:`3`
          (set `self.CurrentStepText` _step3)
          (goto _label))
        (:`4`
          (set `self.CurrentStepText` _step4)
          (goto _label))
        (:`5`
          (set `self.CurrentStepText` _step5)
          (goto _label))
        (:`6`
          (set `self.CurrentStepText` _step6)
          (goto _label))
        (:`7`
          (set `self.CurrentStepText` _step7)
          (goto _label))
        (:`8`
          (set `self.CurrentStepText` _step8)
          (goto _label))
        (:`9`
          (set `self.CurrentStepText` _step9)
          (goto _label))
        (:`10`
          (set `self.CurrentStepText` _step10)
          (goto _label))
        (:`11`
          (set `self.CurrentStepText` _step11)
          (goto _label))
        (:`12`
          (set `self.CurrentStepText` _step12)
          (goto _label))
        (:`13`
          (set `self.CurrentStepText` _step13)
          (goto _label))
        (:`14`
          (set `self.CurrentStepText` _step14)
          (goto _label))
        (:`15`
          (set `self.CurrentStepText` _step15)
          (goto _label))
        (:`16`
          (set `self.CurrentStepText` _step16)
          (goto _label))
        (:`17`
          (set `self.CurrentStepText` _step17)
          (goto _label))
        (:`18`
          (set `self.CurrentStepText` _step18))))))

(fn `UserConstructionScript`)
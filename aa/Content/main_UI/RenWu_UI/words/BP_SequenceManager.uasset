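; BP_SequenceManager is a manager Blueprint that plays a given Level Sequence and records the equipment ID passed with it.
; PlayLevelSequence proceeds only when IsPlaying is already true, then creates a player, binds its finish event, plays it and stores the state.
; OnSequenceFinished clears IsPlaying and checks the BP_TasktipsManager reference, but that branch performs no action.
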(event `PlayLevelSequence`
  (params (SequenceAsset :type "LevelSequence Object Reference") (EquipmentID :type Integer))
  (if (`self.bIsPlaying`)
    (bind (_outactor _returnvalue) (`LevelSequencePlayer.CreateLevelSequencePlayer` SequenceAsset))
    (bind _output_get (set `self.CurrentSequencePlayer1` _returnvalue))
    (add `MovieSceneSequencePlayer.OnFinished` _output_get (delegate `OnSequenceFinished`))
    (`MovieSceneSequencePlayer.Play` (`self.CurrentSequencePlayer1`))
    (set `self.bIsPlaying` true)
    (set `self.CurrentEquipmentID` EquipmentID)))

(event `OnSequenceFinished`
  (set `self.bIsPlaying` false)
  (`/Engine/EditorBlueprintResources/StandardMacros.IsValid` "/Game/main_UI/RenWu_UI/words/BP_TasktipsManager.BP_TasktipsManager"
    (:`Is Valid`
      (if true
        _))))

(fn `UserConstructionScript`)
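; BP_TaskManager1 is a task manager that tracks a list of equipment-interaction steps.
; HandleEquipmentInteract matches equipment and part IDs, or an ordered click sequence for multi-step tasks, then completes the step and plays its Level Sequence through SequenceManagerRef.
; OnSequenceCompleted advances the step or prints an all-done message, and GoToPreviousStep rewinds one.
; UpdateTaskHint only casts the HUD to WBP_TaskPanel2, and the event graph is empty.
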(fn `CompleteCurrentStep`
  (bind _target_sequence (`self.Target Sequence`))
  (set `self.Is Completed` true)
  (`self.UpdateTaskHint`)
  (`/Engine/EditorBlueprintResources/StandardMacros.IsValid` _target_sequence
    (:`Is Valid`
      (if true
        (`/Game/main_UI/RenWu_UI/words/BP_SequenceManager.PlayLevelSequence` (`self.SequenceManagerRef`) _target_sequence (`self.Target Equipment ID`))))))

(fn `ExecuteCurrentStepOperation`
  (bind _returnvalue (- (`self.CurrentTaskStep`) (`self.Promote to Constant`) 0))
  (bind (_stepnumber _taskdescription _targetequipmentid _targetequipmentids _targetpartid _targetsequence _biscompleted) (break `/Game/main_UI/RenWu_UI/words/S_TaskStep` (`|GetArrayItem` (`self.Tasks`) _returnvalue)))
  (if (and (`KismetSystemLibrary.IsValid` _targetsequence) (`KismetArrayLibrary.Array_IsValidIndex` (`|MakeArray` _biscompleted) _returnvalue))
    (`/Game/main_UI/RenWu_UI/words/BP_SequenceManager.PlayLevelSequence` (`self.SequenceManagerRef`) _targetsequence _targetequipmentid)))

(fn `Go to Previous Step`
  (if (> (`self.CurrentTaskStep`) 1)
    (`/Engine/EditorBlueprintResources/StandardMacros.DecrementInt` (`self.CurrentTaskStep`)
      (:`  `
        (set `self.Current Click Index` 0)
        (set `self.Is Completed` false)
        (`self.UpdateTaskHint`)))))

(fn `HandleEquipmentInteract`
  (params (Equipment :type "/Game/UI/BP/interact/BP_l/BP_interact Object Reference") (PartID :type Integer))
  (locals (EquipmentID :type "/Game/UI/BP/interact/BP_l/BP_interact Object Reference") (NewLocalVar :type Boolean))
  (bind (_stepnumber _taskdescription _targetequipmentid _targetequipmentids _targetpartid _targetsequence _biscompleted _bismultistep _currentclickindex) (break `/Game/main_UI/RenWu_UI/words/S_TaskStep` (`|GetArrayItem` (`self.Tasks`) (- (`self.CurrentTaskStep`) 1))))
  (bind _output_get (set `self.Is Completed` _biscompleted))
  (if _output_get
    (return)
    (elif _bismultistep
      (if (== (`/Game/UI/BP/interact/BP_l/BP_interact.EquipmentID` (`self.Equipment`)) (`|GetArrayItem` (stale _output_get_2) _currentclickindex))
        (bind _output_get_2 (set `self.Target Equipment IDs` _targetequipmentids))
        (`/Engine/EditorBlueprintResources/StandardMacros.IncrementFloat` (`KismetMathLibrary.Conv_IntToDouble` _currentclickindex)
          (:`  `
            (if (>= _currentclickindex (`KismetArrayLibrary.Array_Length` _targetequipmentids))
              (`self.CompleteCurrentStep`)
              (else
                (`self.UpdateTaskHint`))))))
      (elif (and (== (`/Game/UI/BP/interact/BP_l/BP_interact.EquipmentID` Equipment) _targetequipmentid) (or (== _targetpartid 0) (== PartID _targetpartid)))
        (`self.CompleteCurrentStep`)))))

(fn `OnSequenceCompleted`
  (`/Engine/EditorBlueprintResources/StandardMacros.IncrementFloat` (`KismetMathLibrary.Conv_IntToDouble` (`self.CurrentTaskStep`))
    (:`  `
      (if (<= (`self.CurrentTaskStep`) (`KismetArrayLibrary.Array_Length` (`self.Tasks`)))
        (`self.UpdateTaskHint`)
        (else
          (`KismetSystemLibrary.PrintString` "所有任务完成，显示结束语"))))))

(fn `UpdateTaskHint`
  (`/Engine/EditorBlueprintResources/StandardMacros.IsValid` (`self.HUDWidgetRef`)
    (:`Is Valid`
      (if true
        (bind _aswbp_task_panel_2 (cast `/Game/main_UI/RenWu_UI/WBP_TaskPanel2` (`self.HUDWidgetRef`)))))))

(fn `UserConstructionScript`)
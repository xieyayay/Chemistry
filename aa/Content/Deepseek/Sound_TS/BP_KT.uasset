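; BP_KT is a trigger actor that toggles an in-world widget and plays air-conditioning room audio (空调房音频).
; Each Box begin overlap, with no filter on the overlapping actor, advances a FlipFlop after validity checks on Box and Widget.
; After a short delay, one branch shows the Widget and plays the sound at world origin, while the other only hides the Widget.
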(event `self.Box.OnComponentBeginOverlap`
  (params (OverlappedComponent :type "PrimitiveComponent Object Reference") (OtherActor :type "Actor Object Reference") (OtherComp :type "PrimitiveComponent Object Reference") (OtherBodyIndex :type Integer) (bFromSweep :type Boolean) (SweepResult :type "HitResult Structure (by ref)"))
  (`/Engine/EditorBlueprintResources/StandardMacros.IsValid` (`self.Box`)
    (:`Is Valid`
      (`self.Widget`
        (:`then`
          (`/Engine/EditorBlueprintResources/StandardMacros.FlipFlop`
            (:`A`
              (`KismetSystemLibrary.Delay` 1.0)
              (`SceneComponent.SetVisibility` (`self.Widget`) true false)
              (`GameplayStatics.PlaySoundAtLocation` "/Game/Deepseek/Sound_TS/空调房音频.空调房音频" (0.0 0.0 0.0) (struct) 1.0 1.0 0.0 null null null null))
            (:`B`
              (`KismetSystemLibrary.Delay` 1.0)
              (`SceneComponent.SetVisibility` (`self.Widget`) false false))))
        (:`else`)))))

(fn `UserConstructionScript`)
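; Sequence manager Blueprint that plays Level Sequences through a PlayLevelSequence event taking a sequence asset and equipment ID.
; The event body runs only when IsPlaying is already true, creating a player, binding its finished callback and starting playback.
; It then sets IsPlaying, which OnSequenceFinished clears.
; CurrentEquipmentID is assigned to itself rather than the EquipmentID input, and TaskManagerRef is unused.
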(event `Play Level Sequence`
  (params (SequenceAsset :type "LevelSequence Object Reference") (EquipmentID :type Integer))
  (if (`self.bIsPlaying`)
    (`LevelSequencePlayer.CreateLevelSequencePlayer` null)
    (`AnimSingleNodeInstance.SetPlaying` false)
    (add `MovieSceneSequencePlayer.OnFinished` (delegate `OnSequenceFinished`))
    (`DatasmithImportedSequencesActor.PlayLevelSequence` "/Game/Anim/1LevelSequence.1LevelSequence")
    (set `self.bIsPlaying` true)
    (set `self.CurrentEquipmentID` (`self.CurrentEquipmentID`))))

(event `OnSequenceFinished`
  (set `self.bIsPlaying` false))

(fn `UserConstructionScript`)
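; Task manager actor that tracks the player's current task and step from the DT_Tasks data table and broadcasts progress to listeners.
; UpdateUI, also run at BeginPlay, picks one of seven step text columns and fires OnTaskUpdated with the title and text.
; AdvanceStep increments the step up to the row's TotalSteps, then calls NextTask.
; NextTask moves through rows using a stored NextIndex, resets the step and conditionally fires OnTaskCompleted.
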(event `self.ReceiveBeginPlay`
  (`self.Update UI`))

(fn `AdvanceStep`
  (bind _returnvalue (`|GetDataTableRow` "/Game/RW_main_UI/RenWu_UI/BP_snd_struct/DT_Tasks.DT_Tasks" (`self.CurrentTaskRow`))
    (:`then`
      (bind (_text _color _tasktitle _step1 _step2 _step3 _step4 _step5 _step6 _step7 _totalsteps) (break `/Game/RW_main_UI/RenWu_UI/BP_snd_struct/Message_Struct` _returnvalue))
      (if (< (`self.CurrentStep`) _totalsteps)
        (set `self.CurrentStep` (+ 1 (`self.CurrentStep`)))
        (`self.Update UI`)
        (return)
        (else
          (if (== (`self.CurrentStep`) _totalsteps)
            _
            (else
              _))
          (`self.NextTask`)
          (`self.Update UI`)
          (return))))))

(fn `NextTask`
  (bind _outrownames (`DataTableFunctionLibrary.GetDataTableRowNames` "/Game/RW_main_UI/RenWu_UI/BP_snd_struct/DT_Tasks.DT_Tasks"))
  (if (< (+ (`KismetArrayLibrary.Array_Find` _outrownames (`self.CurrentTaskRow`)) 1) (`KismetArrayLibrary.Array_Length` _outrownames))
    (set `self.CurrentTaskRow` (`|GetArrayItem` _outrownames (`self.NextIndex`)))
    (set `self.CurrentStep` 1)
    (`self.Update UI`)
    (for (_array_element _array_index) _outrownames
      (if (== _array_element (`self.CurrentTaskRow`))
        (set `self.CurrentTaskIndex` _array_index)
        (break)))
    (bind _result (`/Engine/EditorBlueprintResources/StandardMacros.IncrementFloat` (`KismetMathLibrary.Conv_IntToDouble` (`self.CurrentTaskIndex`)))
      (:`  `
        (bind _output_get (set `self.NextIndex` (`KismetMathLibrary.FTrunc` _result)))
        (if (< _output_get 8.0)
          (`self.OnTaskCompleted` "任务完成！"))))
    (else
      (`KismetSystemLibrary.PrintString` "所有任务已完成"))))

(fn `Update UI`
  (bind _returnvalue (`|GetDataTableRow` "/Game/RW_main_UI/RenWu_UI/BP_snd_struct/DT_Tasks.DT_Tasks" (`self.CurrentTaskRow`))
    (:`then`
      (switch `int` (`self.CurrentStep`)
        (:`1`
          (bind (_text _color _tasktitle _step1 _step2 _step3 _step4 _step5 _step6 _step7) (break `/Game/RW_main_UI/RenWu_UI/BP_snd_struct/Message_Struct` _returnvalue))
          (set `self.CurrentStepText` _step1))
        (:`2`
          (set `self.CurrentStepText` _step2))
        (:`3`
          (set `self.CurrentStepText` _step3))
        (:`4`
          (set `self.CurrentStepText` _step4))
        (:`5`
          (set `self.CurrentStepText` _step5))
        (:`6`
          (set `self.CurrentStepText` _step6))
        (:`7`
          (set `self.CurrentStepText` _step7)))
      (`self.OnTaskUpdated` _tasktitle (`self.CurrentStepText`)))))

(fn `UserConstructionScript`)